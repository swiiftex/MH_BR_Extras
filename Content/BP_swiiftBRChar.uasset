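; Mordhau battle royale player character that adds kill rewards, killstreak abilities and zone-edge feedback.
; A timer polls player-state kills, upgrading the lowest-tier armor slot and granting a UAV at two kills and a Zone Protector at three.
; Slot keys spend streaks: UAV attaches death marks to other living characters, while Zone Protector spawns as held equipment.
; After GameStart, another timer drives the circle-edge widget; deaths spawn a bandage at the killer.
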(event Custom|UAV
  (Audio|PlaySound2D "/BRExtras/Killstreaks/uavactivated.uavactivated" 2.0 1.0 0.0 0 0)
  (bind _outactors (Actor|GetAllActorsOfClass "/Script/Mordhau.MordhauCharacter"))
  (for _array_element _outactors
    (if (not (Class|AdvancedCharacter|GetIsDead _array_element))
      (if (not (== _array_element self))
        (bind _returnvalue (Game|SpawnActorfromClass "/BRExtras/Killstreaks/BP_DeathMark.BP_DeathMark_C" (Transformation|GetActorTransform _array_element) "Undefined" 0 _array_element (Variables|Default|GetUAVLength) 0))
        (Transformation|AttachActorToActor _returnvalue _array_element "None" "SnapToTarget" "SnapToTarget" "SnapToTarget" true))))
  (bind _foundwidgets (Widget|GetAllWidgetsOfClass "/BRExtras/BP_BattleRoyaleHUDWidget_Extras.BP_BattleRoyaleHUDWidget_Extras_C" false))
  (Default|ShowKillstreak (Utilities|Array|Get(acopy) _foundwidgets) "UAV Active!" (Variables|Default|GetUAVLength))
  (CallFunction|AllAnnouncement (Utilities|Text|FormatText "{a} activated a UAV!" (PlayerState|GetPlayerName (Variables|Default|GetPlayerState)))))

(event Custom|CustomEvent_0
  (bind _localplayerstate (Variables|Default|GetLocalPlayerState))
  (bind _kills (Variables|/Script/Mordhau.MordhauPlayerState|GetKills _localplayerstate))
  (Development|PrintText (Utilities|Text|FormatText "{b} has {a} kills" (PlayerState|GetPlayerName _localplayerstate) _kills))
  (if (Variables|/Script/Mordhau.MordhauPlayerState|GetbIsAlive _localplayerstate)
    (Utilities|FlowControl|Sequence
      (:then_0
        (if (> _kills (Variables|Default|GetLastObservedKills))
          (Variables|Default|SetLastObservedKills _kills)
          (CallFunction|UpgradeArmor)
          (switch int _kills
            (:2
              (Utilities|FlowControl|DoOnce false
                (:Completed
                  (CallFunction|GiveKillstreak "UAV" _kills "/BRExtras/Killstreaks/uav_cue.uav_cue"))))
            (:3
              (Utilities|FlowControl|DoOnce false
                (:Completed
                  (CallFunction|GiveKillstreak "Zone" _kills "/BRExtras/ZoneProtector/emp_Cue.emp_Cue")))))))
      (:then_1
        (if (== (Variables|Default|GetHeadArmor) "/BRExtras/CustomCosmetics/Rat/BP_RatHelmetPickup.BP_RatHelmetPickup_C")
          (CallFunction|GiveRatHelm))))))

(event Custom|ServerTimer
  (bind _returnvalue (Utilities|Time|SetTimerbyFunctionName 0 "CheckForGameStart" 1.0 true))
  (Variables|Default|SetGameStartCheckTimer _returnvalue))

(event Custom|CLI%20Remove%20Circle%20Effect
  (bind _foundwidgets (Widget|GetAllWidgetsOfClass "/BRExtras/W_CircleEffect.W_CircleEffect_C" false))
  (for _array_element _foundwidgets
    (Widget|RemovefromParent _array_element))
  (Development|PrintString "REMOVED ALL CIRCLE EFFECTS" true true "(R=1.000000,G=0.000000,B=0.077258,A=1.000000)"))

(event Custom|CLI%20Add%20Circle%20Effect
  (bind _returnvalue (UserInterface|CreateWidget "/BRExtras/W_CircleEffect.W_CircleEffect_C"))
  (UserInterface|Viewport|AddtoViewport _returnvalue -1)
  (Variables|Default|SetCircleEffect _returnvalue)
  (Development|PrintString "ADDED CIRCLE EFFECT" true true "(R=0.409041,G=1.000000,B=0.000000,A=1.000000)"))

(event Custom|CLI%20Tick
  (if (Variables|Default|GetGameStarted)
    (bind _returnvalue (CallFunction|GetDistancetoCircleEdge))
    (if (< (Math|Float|Absolute(Float) _returnvalue) 1e+02)
      (Utilities|IsValid (Variables|Default|GetCircleEffect)
        (:Is%20Valid
          _)
        (:Is%20Not%20Valid
          (bind _returnvalue_2 (UserInterface|CreateWidget "/BRExtras/W_CircleEffect.W_CircleEffect_C"))
          (UserInterface|Viewport|AddtoViewport _returnvalue_2 -10)
          (Variables|Default|SetCircleEffect _returnvalue_2)
          (Development|PrintString "ADDED CIRCLE EFFECT" true true "(R=0.409041,G=1.000000,B=0.000000,A=1.000000)")))
      (Default|UpdateZoneDistance (Variables|Default|GetCircleEffect) _returnvalue)
      (Default|SetinZone (Variables|Default|GetCircleEffect) (Utilities|Set|Contains (Variables|/Game/Mordhau/Blueprints/GameModes/BattleRoyale/BP_BattleRoyaleCircle.BP_BattleRoyaleCircle_C|GetUnsafeCharacters (Variables|Default|GetBR%20Circle%20Ref)) self)))))

(event Custom|UpgradeArmorClient
  (bind _foundwidgets (Widget|GetAllWidgetsOfClass "/BRExtras/BP_BattleRoyaleHUDWidget_Extras.BP_BattleRoyaleHUDWidget_Extras_C" false))
  (UserInterface|Animation|PlayAnimation (Utilities|Array|Get(acopy) _foundwidgets) (Variables|/BRExtras/BP_BattleRoyaleHUDWidget_Extras.BP_BattleRoyaleHUDWidget_Extras_C|GetUpgradeArmor (Utilities|Array|Get(acopy) _foundwidgets)) 0.0 1 "Forward" 1.0 false))

(event Custom|CLI%20Show%20Timer
  (params (Text :type Text) (Duration :type Float%20%28single-precision%29))
  (bind _foundwidgets (Widget|GetAllWidgetsOfClass "/BRExtras/BP_BattleRoyaleHUDWidget_Extras.BP_BattleRoyaleHUDWidget_Extras_C" false))
  (Default|ShowKillstreak (Utilities|Array|Get(acopy) _foundwidgets) Text Duration))

(event Custom|MC%20Modify%20attack
  (bind _returnvalue (Class|AdvancedCharacter|GetMotion))
  (if (Variables|Default|GetbCannotChamber)
    (bind _asstrike_motion (Utilities|Casting|CastToStrikeMotion _returnvalue)
      (:then
        (Variables|/Script/Mordhau.AttackMotion|SetMorphWindow _asstrike_motion 999.0)
        (Development|PrintString "Modified strike"))
      (:CastFailed
        (bind _asstab_motion (Utilities|Casting|CastToStabMotion _returnvalue))
        (Variables|/Script/Mordhau.AttackMotion|SetMorphWindow _asstab_motion 999.0)
        (Variables|/Script/Mordhau.AttackMotion|SetFeintWindow _asstab_motion 999.0)
        (Development|PrintString "Modified stab")))))

(event Custom|MC%20Set%20Alt%20Combat
  (params (? :type Boolean))
  (bind _output_get (Variables|Default|SetbCannotChamber ?))
  (if _output_get
    (Utilities|Time|SetTimerbyFunctionName 0 "ModifyEquipmentAltCombat" 1.0 true)))

(event Custom|Start%20Kill%20Checker
  (bind _asbp_battle_royale_player_state (Utilities|Casting|CastToBP_BattleRoyalePlayerState (Variables|Default|GetPlayerState) :!label _label)
    (:then
      (Variables|Default|SetLocalPlayerState _asbp_battle_royale_player_state)
      (Utilities|Time|SetTimerbyEvent (delegate Custom|CustomEvent_0) 1.0 true))
    (:CastFailed
      (Utilities|FlowControl|Delay 1.0)
      (goto _label))))

(event Custom|All%20Announcement
  (params (Text :type Text))
  (bind _asbp_battle_royale_game_mode (Utilities|Casting|CastToBP_BattleRoyaleGameMode (Game|GetGameMode)))
  (Class|MordhauGameMode|Broadcast _asbp_battle_royale_game_mode 0 (Utilities|String|ToString(Text) Text) "ServerSay"))

(event Custom|Attempt%20Activate%20Killstreak
  (params (Selection :type String))
  (switch string Selection
    (:UAV
      (if (Variables|Default|GetHasUAV)
        (CallFunction|UAV)
        (Variables|Default|SetHasUAV false)
        (bind _foundwidgets (Widget|GetAllWidgetsOfClass "/BRExtras/BP_BattleRoyaleHUDWidget_Extras.BP_BattleRoyaleHUDWidget_Extras_C" false))
        (Default|KillstreakUsed (Utilities|Array|Get(acopy) _foundwidgets) "UAV")))
    (:Zone
      (if (Variables|Default|GetHasZoneProt)
        (CallFunction|ZoneProtector)
        (Variables|Default|SetHasZoneProt false)
        (bind _foundwidgets_2 (Widget|GetAllWidgetsOfClass "/BRExtras/BP_BattleRoyaleHUDWidget_Extras.BP_BattleRoyaleHUDWidget_Extras_C" false))
        (Default|KillstreakUsed (Utilities|Array|Get(acopy) _foundwidgets_2) "Zone Protector")))))

(event Custom|Give%20Killstreak
  (params (Streak :type String) (Kills :type Integer) (Sound :type Sound%20Cue%20Object%20Reference))
  (switch string Streak
    (:UAV
      (Variables|Default|SetHasUAV true)
      (bind _foundwidgets (Widget|GetAllWidgetsOfClass "/BRExtras/BP_BattleRoyaleHUDWidget_Extras.BP_BattleRoyaleHUDWidget_Extras_C" false))
      (Default|KillstreakEarned (Utilities|Array|Get(acopy) _foundwidgets) Kills "UAV" Sound))
    (:Zone
      (Variables|Default|SetHasZoneProt true)
      (bind _foundwidgets_2 (Widget|GetAllWidgetsOfClass "/BRExtras/BP_BattleRoyaleHUDWidget_Extras.BP_BattleRoyaleHUDWidget_Extras_C" false))
      (Default|KillstreakEarned (Utilities|Array|Get(acopy) _foundwidgets_2) Kills "Zone Protector" Sound))))

(event Custom|ZoneProtector
  (bind _returnvalue (Game|SpawnActorfromClass "/BRExtras/ZoneProtector/BP_ZoneProtector.BP_ZoneProtector_C" (Transformation|GetActorTransform) "Undefined" 0 0))
  (Class|MordhauCharacter|FreeHandsforEquipment _returnvalue)
  (Class|MordhauCharacter|SwitchEquipment _returnvalue))

(event Custom|GiveRatHelm
  (Rendering|SetVisibility (Variables|Default|Getrathelmet) true false)
  (Development|PrintString "Rat helm user"))

(event Custom|Game%20Start
  (Utilities|FlowControl|Delay 2.0)
  (bind _returnvalue (Actor|GetActorOfClass "/Game/Mordhau/Blueprints/GameModes/BattleRoyale/BP_BattleRoyaleCircle.BP_BattleRoyaleCircle_C"))
  (Variables|Default|SetBR%20Circle%20Ref _returnvalue)
  (Variables|Default|SetGameStarted true)
  (Utilities|Time|SetTimerbyEvent (delegate Custom|CLI%20Tick) 0.05 true))

(event Custom|UpgradeArmor
  (bind (_value _returnvalue) (CallFunction|GetUpgradedArmorClass))
  (if _returnvalue
    (bind _returnvalue_2 (Game|SpawnActorfromClass _value (Transformation|GetActorTransform) "AlwaysSpawn" 0 0))
    (Utilities|FlowControl|Delay 0.2)
    (Default|Equip _returnvalue_2 self)
    (CallFunction|UpgradeArmorClient)))

(event EventOnKilled
  (params (EventInstigator :type Controller%20Object%20Reference))
  (CallFunction|CLIRemoveCircleEffect)
  (bind _returnvalue (Game|SpawnActorfromClass "/Game/Mordhau/Blueprints/Equipment/BP_EquipmentSpawner.BP_EquipmentSpawner_C" (Transformation|GetActorTransform (Pawn|GetControlledPawn EventInstigator)) "AdjustIfPossibleButAlwaysSpawn" 0 0))
  (Variables|/Game/Mordhau/Blueprints/Equipment/BP_EquipmentSpawner.BP_EquipmentSpawner_C|SetEquipment _returnvalue "/Game/Mordhau/Blueprints/Equipment/Misc/BP_Bandage_BR_2.BP_Bandage_BR_2_C")
  (Default|SpawnEquipment _returnvalue)
  (Actor|DestroyActor _returnvalue)
  (|CallParentFunction EventInstigator))

(event EventPossessed
  (params (NewController :type Controller%20Object%20Reference))
  (|CallParentFunction NewController)
  (Utilities|FlowControl|Delay 5.0)
  (if (Pawn|IsPlayerControlled)
    (CallFunction|StartKillChecker)))

(event EventBeginPlay
  (|CallParentFunction))

(event Input|ActionEvents|InputActionEquipSlot8
  (params (Key :type Key%20Structure :default "None"))
  (:Pressed
    (CallFunction|AttemptActivateKillstreak "Zone")))

(event Input|ActionEvents|InputActionEquipSlot7
  (params (Key :type Key%20Structure :default "None"))
  (:Pressed
    (CallFunction|AttemptActivateKillstreak "UAV")))

(fn ConstructionScript
  (|CallParentFunction))

(fn CheckforGameStart
  (bind _asbp_battle_royale_game_state (Utilities|Casting|CastToBP_BattleRoyaleGameState (Game|GetGameState)))
  (if (not (Variables|/Game/Mordhau/Blueprints/GameModes/BP_MordhauGameState.BP_MordhauGameState_C|GetMatchEndInfoReplicated _asbp_battle_royale_game_state))
    (Utilities|FlowControl|DoOnce false
      (:Completed
        (Utilities|Time|ClearandInvalidateTimerbyHandle (Variables|Default|GetGameStartCheckTimer))
        (CallFunction|GameStart)))))

(fn GetDistancetoCircleEdge
  (bind _br_circle_ref (Variables|Default|GetBR%20Circle%20Ref))
  (bind _capsule (Variables|/Game/Mordhau/Blueprints/GameModes/BattleRoyale/BP_BattleRoyaleCircle.BP_BattleRoyaleCircle_C|GetCapsule _br_circle_ref))
  (Utilities|IsValid _br_circle_ref
    (:Is%20Valid
      (return (- (Math|Vector|VectorLengthXY (- (Transformation|GetWorldLocation _capsule) (Transformation|GetActorLocation (Pawn|GetControlledPawn (Game|GetPlayerController 0))))) (Components|Capsule|GetScaledCapsuleRadius _capsule))))
    (:Is%20Not%20Valid
      (Development|PrintString "WARNING CIRCLE NOT VALID"))))

(fn GetUpgradedArmorClass
  (bind _asbp_wearable_pickup (Utilities|Casting|CastToBP_WearablePickup (Class|MordhauUtilityLibrary|GetDefaultActor (Variables|Default|GetLegArmor)))
    (:then
      (LocalVariables|SetLowestTier (Variables|/Game/Mordhau/Blueprints/Interactables/WearablePickups/BP_WearablePickup.BP_WearablePickup_C|GetTier _asbp_wearable_pickup)))
    (:CastFailed
      (LocalVariables|SetLowestTier 0)))
  (LocalVariables|SetLowestTierSlot "Legs")
  (bind _asbp_wearable_pickup_2 (Utilities|Casting|CastToBP_WearablePickup (Class|MordhauUtilityLibrary|GetDefaultActor (Variables|Default|GetHeadArmor)))
    (:then
      (if (<= (Variables|/Game/Mordhau/Blueprints/Interactables/WearablePickups/BP_WearablePickup.BP_WearablePickup_C|GetTier _asbp_wearable_pickup_2) (LocalVariables|GetLowestTier))
        (LocalVariables|SetLowestTier (Variables|/Game/Mordhau/Blueprints/Interactables/WearablePickups/BP_WearablePickup.BP_WearablePickup_C|GetTier _asbp_wearable_pickup_2))
        (LocalVariables|SetLowestTierSlot "Head" :!label _label)))
    (:CastFailed
      (LocalVariables|SetLowestTier 0)
      (goto _label)))
  (bind _asbp_wearable_pickup_3 (Utilities|Casting|CastToBP_WearablePickup (Class|MordhauUtilityLibrary|GetDefaultActor (Variables|Default|GetChestArmor)))
    (:then
      (if (<= (Variables|/Game/Mordhau/Blueprints/Interactables/WearablePickups/BP_WearablePickup.BP_WearablePickup_C|GetTier _asbp_wearable_pickup_3) (LocalVariables|GetLowestTier))
        (LocalVariables|SetLowestTier (Variables|/Game/Mordhau/Blueprints/Interactables/WearablePickups/BP_WearablePickup.BP_WearablePickup_C|GetTier _asbp_wearable_pickup_3))
        (LocalVariables|SetLowestTierSlot "UpperChest" :!label _label_2)))
    (:CastFailed
      (LocalVariables|SetLowestTier 0)
      (goto _label_2)))
  (if (< (LocalVariables|GetLowestTier) 3)
    (return (.Value (Utilities|Map|Find (Utilities|Select :Index (LocalVariables|GetLowestTierSlot) :Head (LocalVariables|GetHeadArmors) :Coif 0 :UpperChest (LocalVariables|GetChestArmors) :LowerChest 0 :Shoulders 0 :Arms 0 :Hands 0 :Legs (LocalVariables|GetLegArmors) :Feet 0 :Total 0 :Invalid 0) (+ (LocalVariables|GetLowestTier) 1))) (.ReturnValue (Utilities|Map|Find (Utilities|Select :Index (LocalVariables|GetLowestTierSlot) :Head (LocalVariables|GetHeadArmors) :Coif 0 :UpperChest (LocalVariables|GetChestArmors) :LowerChest 0 :Shoulders 0 :Arms 0 :Hands 0 :Legs (LocalVariables|GetLegArmors) :Feet 0 :Total 0 :Invalid 0) (+ (LocalVariables|GetLowestTier) 1))))
    (else
      (return 0 false))))