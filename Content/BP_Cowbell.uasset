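; BP_Cowbell is a 20-second marker that flags its owning Mordhau character as a hiding player.
; It retries the owner cast until valid, then shows that local player a "Marked for death!" killstreak message and hides its widget.
; For everyone else, it attaches to the character, displays "{name} is hiding!" and rings a bell periodically.
; Timed and on-destroy death checks spawn an airdrop at its location if the marked player is dead.
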(event Custom|ServerCheckAlive
  (if (Variables|/Script/Mordhau.AdvancedCharacter|GetbIsDead (Variables|Default|GetAs%20Mordhau%20Character))
    (Utilities|FlowControl|DoOnce false
      (:Completed
        (Game|SpawnActorfromClass "/BRExtras/Airdrops/BP_swiiftAirdrop.BP_swiiftAirdrop_C" (Transformation|GetActorTransform) "AdjustIfPossibleButAlwaysSpawn" 0 3.0 0)
        (Actor|DestroyActor)))))

(event EventBeginPlay
  (Actor|SetLifeSpan 2e+01)
  (bind _asmordhau_character (Utilities|Casting|CastToMordhauCharacter (Components|GetOwner self) :!label _label)
    (:then
      (bind _output_get (Variables|Default|SetAs%20Mordhau%20Character _asmordhau_character))
      (if (== (Game|GetPlayerController 0) (Pawn|GetController _output_get))
        (Rendering|SetVisibility (Variables|Default|GetWidget) false true)
        (bind _foundwidgets (Widget|GetAllWidgetsOfClass "/BRExtras/BP_BattleRoyaleHUDWidget_Extras.BP_BattleRoyaleHUDWidget_Extras_C" false))
        (Default|ShowKillstreak (Utilities|Array|Get(acopy) _foundwidgets) "Marked for death!" 2e+01)
        (else
          (Transformation|AttachComponentToComponent (Variables|/Script/Engine.Character|GetCapsuleComponent _output_get) "None" "SnapToTarget" "SnapToTarget" "SnapToTarget" false)
          (Utilities|Time|SetTimerbyFunctionName 0 "PlayAudio" 3.0 true)
          (Utilities|Time|SetTimerbyEvent (delegate Custom|ServerCheckAlive) 0.5 true)
          (bind _asw_pussy (Utilities|Casting|CastToW_Pussy (UserInterface|GetWidget (Variables|Default|GetWidget))))
          (Rendering|Components|TextRender|SetText (Variables|/BRExtras/Killstreaks/W_Pussy.W_Pussy_C|GetTextBlock_236 _asw_pussy) (Utilities|Text|FormatText "{name} is hiding!" (PlayerState|GetPlayerName (Variables|/Script/Engine.Pawn|GetPlayerState _output_get)))))))
    (:CastFailed
      (Utilities|FlowControl|Delay 1.0)
      (goto _label))))

(event EventDestroyed
  (CallFunction|ServerCheckAlive))

(fn ConstructionScript)

(fn PlayAudio
  (bind _as_mordhau_character (Variables|Default|GetAs%20Mordhau%20Character))
  (CallFunction|ServerCheckAlive)
  (Utilities|IsValid _as_mordhau_character
    (:Is%20Valid
      (Audio|SpawnSoundAttached "/Game/Mordhau/Audio/Cues/Instruments/Bell.Bell" (Variables|/Script/Engine.Character|GetCapsuleComponent _as_mordhau_character) "None" "0, 0, 0" "0, 0, 0" "KeepRelativeOffset" false 1.0 1.0 0.0 0 0))
    (:Is%20Not%20Valid
      (Actor|DestroyActor))))