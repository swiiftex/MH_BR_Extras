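; Battle Royale statue interactable that blesses a player's held weapon when their kill count meets the cost.
; A held interaction adds a blessing component to the first unblessed right- or left-hand equipment, records the player and plays particle and sound effects.
; Remote clients poll on a timer to refresh prompt text and interactability from local equipment and prior use.
; UpdateVisuals instead checks Horde coins for affordability, plus camera distance for visibility.
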(event Custom|BlessingEffectsMulti
  (bind _interacteffectlocation (Variables|Default|GetInteractEffectLocation))
  (bind _returnvalue (Transformation|GetWorldLocation _interacteffectlocation))
  (Utilities|FlowControl|Sequence
    (:then_0
      (CallFunction|UpdateInteractText))
    (:then_1
      (Effects|SpawnEmitteratLocation "/Game/Mordhau/Assets/Environment/Horde_DemonInvasion/PackAPunch/P_StatueInteract.P_StatueInteract" _returnvalue)
      (Audio|PlaySoundatLocation "/Game/Mordhau/Audio/Cues/Horde/Abilities/Soundcues/SC_Blessing_DIH.SC_Blessing_DIH" _returnvalue "0, 0, 0" 1.0 1.0 0.0 0 0 0))))

(event Custom|CheckCanInteract
  (CallFunction|UpdateInteractText)
  (if (Utilities|Enum|Equal(Enum) (Variables|Default|GetInteractionText) (Utilities|Text|MakeLiteralText "Unable to Apply Blessing"))
    (Variables|Default|SetbIsInteractable false)
    (else
      (Variables|Default|SetbIsInteractable true))))

(event EventOnHighlightStart
  (|CallParentFunction)
  (CallFunction|UpdateInteractText))

(event EventBeginPlay
  (|CallParentFunction)
  (Audio|PlaySoundatLocation "/Game/Mordhau/Audio/Cues/Horde/Abilities/Soundcues/SC_Blessing_Loop_DIH.SC_Blessing_Loop_DIH" (Transformation|GetActorLocation) "0, 0, 0" 1.0 1.0 0.0 0 0 0)
  (Networking|SwitchHasAuthority
    (:Remote
      (Utilities|Time|SetTimerbyEvent (delegate Custom|CheckCanInteract) 0.25 true))))

(event EventOnHeldInteractionStart
  (params (Character :type Mordhau%20Character%20Object%20Reference))
  (bind _righthandequipment (Variables|/Script/Mordhau.MordhauCharacter|GetRightHandEquipment Character))
  (bind _lefthandequipment (Variables|/Script/Mordhau.MordhauCharacter|GetLeftHandEquipment Character))
  (|CallParentFunction Character)
  (bind _asbp_battle_royale_player_state (Utilities|Casting|CastToBP_BattleRoyalePlayerState (Variables|/Script/Engine.Pawn|GetPlayerState Character)))
  (if (>= (Variables|/Script/Mordhau.MordhauPlayerState|GetKills _asbp_battle_royale_player_state) (Variables|Default|GetCost))
    (Utilities|FlowControl|Sequence
      (:then_0
        (Utilities|IsValid _righthandequipment
          (:Is%20Valid
            (Utilities|IsValid (Actor|GetComponentbyClass _righthandequipment "/Game/Mordhau/Blueprints/GameModes/Horde/DemonInvasion/Blessings/BP_BlessingComponent.BP_BlessingComponent_C")
              (:Is%20Valid
                (Utilities|IsValid _lefthandequipment :!label _label
                  (:Is%20Valid
                    (Utilities|IsValid (Actor|GetComponentbyClass _lefthandequipment "/Game/Mordhau/Blueprints/GameModes/Horde/DemonInvasion/Blessings/BP_BlessingComponent.BP_BlessingComponent_C")
                      (:Is%20Valid
                        _)
                      (:Is%20Not%20Valid
                        (AddComponent|AddBPBlessingComponent _lefthandequipment))))))
              (:Is%20Not%20Valid
                (AddComponent|AddBPBlessingComponent _righthandequipment))))
          (:Is%20Not%20Valid
            (goto _label)))
        (Utilities|Array|Add (Variables|Default|GetPlayersAlreadyUsed) _asbp_battle_royale_player_state))
      (:then_1
        (CallFunction|BlessingEffectsMulti)))))

(fn ConstructionScript
  (|CallParentFunction))

(fn UpdateInteractText
  (if (== (Utilities|Array|FindItem (Variables|Default|GetPlayersAlreadyUsed) (Variables|/Script/Engine.Controller|GetPlayerState (Game|GetPlayerController 0))) -1)
    (Utilities|FlowControl|Sequence
      (:then_0
        (LocalVariables|SetCurrentEquipment "NONE")
        (bind _asbp_mordhau_character (Utilities|Casting|CastToBP_MordhauCharacter (Pawn|GetControlledPawn (Game|GetPlayerController 0))))
        (Utilities|IsValid (Variables|/Script/Mordhau.MordhauCharacter|GetRightHandEquipment _asbp_mordhau_character)
          (:Is%20Valid
            (Utilities|IsValid (Actor|GetComponentbyClass (Variables|/Script/Mordhau.MordhauCharacter|GetRightHandEquipment _asbp_mordhau_character) "/Game/Mordhau/Blueprints/GameModes/Horde/DemonInvasion/Blessings/BP_BlessingComponent.BP_BlessingComponent_C")
              (:Is%20Valid
                (Utilities|IsValid (Variables|/Script/Mordhau.MordhauCharacter|GetLeftHandEquipment _asbp_mordhau_character) :!label _label
                  (:Is%20Valid
                    (Utilities|IsValid (Actor|GetComponentbyClass (Variables|/Script/Mordhau.MordhauCharacter|GetLeftHandEquipment _asbp_mordhau_character) "/Game/Mordhau/Blueprints/GameModes/Horde/DemonInvasion/Blessings/BP_BlessingComponent.BP_BlessingComponent_C")
                      (:Is%20Not%20Valid
                        (LocalVariables|SetCurrentEquipment (Variables|/Script/Mordhau.MordhauEquipment|GetEquipmentName (Variables|/Script/Mordhau.MordhauCharacter|GetLeftHandEquipment _asbp_mordhau_character))))))))
              (:Is%20Not%20Valid
                (LocalVariables|SetCurrentEquipment (Variables|/Script/Mordhau.MordhauEquipment|GetEquipmentName (Variables|/Script/Mordhau.MordhauCharacter|GetRightHandEquipment _asbp_mordhau_character))))))
          (:Is%20Not%20Valid
            (goto _label))))
      (:then_1
        (if (Utilities|Enum|Equal(Enum) (Utilities|Text|MakeLiteralText "NONE") (LocalVariables|GetCurrentEquipment))
          (Variables|Default|SetInteractionText "Unable to Apply Blessing")
          (else
            (Variables|Default|SetInteractionText (Utilities|Text|FormatText "Bless {Equipment}" (LocalVariables|GetCurrentEquipment)))))))
    (else
      (Variables|Default|SetInteractionText "Already used"))))

(fn UpdateVisuals
  (bind _returnvalue (Math|Float|MakeLiteralFloat 8e+02))
  (bind _returnvalue_2 (Game|GetPlayerCameraManager 0))
  (bind _returnvalue_3 (Transformation|GetActorLocation))
  (bind _returnvalue_4 (Game|GetPlayerController 0))
  (bind _returnvalue_5 (Camera|GetCameraLocation _returnvalue_2))
  (bind _returnvalue_6 (- _returnvalue_3 _returnvalue_5))
  (bind _returnvalue_7 (Math|Vector|VectorLength _returnvalue_6))
  (Utilities|FlowControl|Sequence
    (:then_0
      (Utilities|IsValid _returnvalue_4
        (:Is%20Valid
          (if (Pawn|IsLocalPlayerController _returnvalue_4)
            (Utilities|FlowControl|Sequence
              (:then_0
                (bind _asbp_horde_player_state (Utilities|Casting|CastToBP_HordePlayerState (Variables|/Script/Engine.Controller|GetPlayerState _returnvalue_4)))
                (LocalVariables|SetCanAffordTemp (>= (Variables|/Game/Mordhau/Blueprints/GameModes/Horde/BP_HordePlayerState.BP_HordePlayerState_C|GetCoins _asbp_horde_player_state) (Variables|Default|GetCost))))
              (:then_1
                (if (< _returnvalue_7 (+ _returnvalue 25.0))
                  (if (< _returnvalue_7 _returnvalue)
                    (LocalVariables|SetCanSeeTemp true))
                  (else
                    (LocalVariables|SetCanSeeTemp false)))))))))
    (:then_1
      (return (LocalVariables|GetCanAffordTemp) (LocalVariables|GetCanSeeTemp)))))