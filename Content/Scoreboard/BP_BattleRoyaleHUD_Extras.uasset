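; Mordhau battle royale HUD Blueprint that adds an Extras overlay widget and scoreboard on top of its parent HUD.
; When game state replicates, it creates the overlay and toggles its visibility with minimal/full HUD and main menu events.
; ShowScoreboard lazily creates the Extras scoreboard while the HUD is visible, limiting it to spectators if the game state disables scoreboards.
; End screen logic is disconnected, leaving ShowBattleRoyaleEndScreen empty.
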(event EventBeginPlay
  (|CallParentFunction))

(event EventOnGameStateReplicated
  (|CallParentFunction)
  (bind _returnvalue (UserInterface|CreateWidget "/BRExtras/BP_BattleRoyaleHUDWidget_Extras.BP_BattleRoyaleHUDWidget_Extras_C" (Game|GetPlayerController 0)))
  (bind _output_get (Variables|Default|SetBattleRoyaleHUDWidget _returnvalue))
  (UserInterface|Viewport|AddtoViewport _output_get -5)
  (if (Variables|Default|GetIsHUDMinimal)
    (Widget|SetVisibility _returnvalue "Collapsed")))

(event EventHideMainMenu
  (|CallParentFunction)
  (Widget|SetVisibility (Variables|Default|GetBattleRoyaleHUDWidget) "Visible"))

(event EventShowMainMenu
  (|CallParentFunction)
  (Widget|SetVisibility (Variables|Default|GetBattleRoyaleHUDWidget) "Collapsed"))

(event EventUseMinimalHUD
  (|CallParentFunction)
  (Utilities|IsValid (Variables|Default|GetBattleRoyaleHUDWidget)
    (:Is%20Valid
      (Widget|SetVisibility (Variables|Default|GetBattleRoyaleHUDWidget) "Collapsed"))))

(event EventUseFullHUD
  (|CallParentFunction)
  (Utilities|IsValid (Variables|Default|GetBattleRoyaleHUDWidget)
    (:Is%20Valid
      (Widget|SetVisibility (Variables|Default|GetBattleRoyaleHUDWidget) "Visible"))))

(fn ConstructionScript
  (|CallParentFunction))

(fn ShowBattleRoyaleEndScreen)

(fn ShowScoreboard
  (bind _asmordhau_game_state (Utilities|Casting|CastToMordhauGameState (Game|GetGameState)))
  (if (Variables|/Script/Mordhau.MordhauGameState|GetbDisableScoreboard _asmordhau_game_state)
    (Utilities|IsValid (Pawn|GetSpectatorPawn (Game|GetPlayerController 0))
      (:Is%20Valid
        _)))
  (if (Widget|IsVisible (Variables|Default|GetHUD))
    (Utilities|IsValid (Variables|Default|GetScoreboard)
      (:Is%20Valid
        (Default|Show (Variables|Default|GetScoreboard)))
      (:Is%20Not%20Valid
        (Utilities|FlowControl|Sequence
          (:then_0
            (bind _returnvalue (UserInterface|CreateWidget "/BRExtras/Scoreboard/BP_BattleRoyaleScoreboard_Extras.BP_BattleRoyaleScoreboard_Extras_C" (Game|GetPlayerController 0)))
            (Variables|Default|SetScoreboard _returnvalue))
          (:then_1
            (Utilities|IsValid (Variables|Default|GetScoreboard)
              (:Is%20Valid
                (Default|Show (Variables|Default|GetScoreboard))
                (Widget|Panel|AddChild (Variables|/Game/Mordhau/UI/BP_HUDWidget.BP_HUDWidget_C|GetScoreboardContainer (Variables|Default|GetHUD)) (Variables|Default|GetScoreboard))))))))))