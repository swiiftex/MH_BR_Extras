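; BP_BRStatTracker tracks per-player win counts for the Battle Royale mode and relays server announcements.
; PlayerWins is an array of player and win pairs whose OnRep rebuilds the WinsMap lookup, working around maps not replicating.
; AllAnnouncement passes text to BP_BattleRoyaleGameMode's Broadcast as a ServerSay message, acting only where that game mode is available.
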(event Custom|All%20Announcement
  (params (Text :type Text))
  (bind _asbp_battle_royale_game_mode (Utilities|Casting|CastToBP_BattleRoyaleGameMode (Game|GetGameMode)))
  (Class|MordhauGameMode|Broadcast _asbp_battle_royale_game_mode 0 (Utilities|String|ToString(Text) Text) "ServerSay"))

(fn ConstructionScript)

(fn OnRepPlayerWins
  (Utilities|Map|Clear (LocalVariables|GetTempWinMap))
  (for _array_element (Variables|Default|GetPlayerWins)
    (Utilities|Map|Add (LocalVariables|GetTempWinMap) (.Player (Utilities|Struct|BreakS_PlayerWins _array_element)) (.Wins (Utilities|Struct|BreakS_PlayerWins _array_element))))
  (Variables|Default|SetWinsMap (LocalVariables|GetTempWinMap)))