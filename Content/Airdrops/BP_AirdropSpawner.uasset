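; Battle Royale airdrop spawner that drops a configurable number of airdrops at timed intervals, with server chat announcements.
; On BeginPlay it reads interval and amount from custom config, tries to spawn a navmesh volume if none exists, and polls for match start.
; Timers then spawn each drop at a location forcer actor if present, otherwise at a random navigable point within the next level's circle.
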(event Custom|All%20Announcement
  (params (Text :type Text))
  (Class|MordhauGameMode|Broadcast (Variables|Default|GetAs%20BP%20Battle%20Royale%20Game%20Mode) 0 (Utilities|String|ToString(Text) Text) "ServerSay"))

(event Custom|SRV%20Airdrop
  (bind _location (CallFunction|GenerateAirdropLocation))
  (CallFunction|SpawnAirdrop _location))

(event EventBeginPlay
  (bind (_isvalid _returnvalue) (Class|MordhauUtilityLibrary|GetCustomConfigVarInt "Airdrops" "Amount"))
  (bind (_isvalid_2 _returnvalue_2) (Class|MordhauUtilityLibrary|GetCustomConfigVarFloat "Airdrops" "DropInterval"))
  (Utilities|FlowControl|Sequence
    (:then_0
      (bind _asbp_battle_royale_game_mode (Utilities|Casting|CastToBP_BattleRoyaleGameMode (Game|GetGameMode)))
      (Variables|Default|SetAs%20BP%20Battle%20Royale%20Game%20Mode _asbp_battle_royale_game_mode)
      (bind _returnvalue_3 (Utilities|Time|SetTimerbyFunctionName 0 "CheckForStart" 1.0 true))
      (Variables|Default|SetCheckerTimer _returnvalue_3)
      (bind _returnvalue_4 (Actor|GetActorOfClass "/Script/NavigationSystem.NavMeshBoundsVolume"))
      (Utilities|IsValid _returnvalue_4 ; If theres no navmeshvolume, generate one
        (:Is%20Not%20Valid
          (bind _returnvalue_5 (Actor|GetActorOfClass "/Game/Mordhau/Blueprints/Characters/BP_MordhauCharacter.BP_MordhauCharacter_C"))
          (bind _asnav_mesh_bounds_volume (Utilities|Casting|CastToNavMeshBoundsVolumeClass "/Script/NavigationSystem.NavMeshBoundsVolume"))
          (Game|SpawnActorfromClass _asnav_mesh_bounds_volume (Math|Transform|MakeTransform (Transformation|GetActorLocation _returnvalue_5) "0, 0, 0" "3000.000000,3000.000000,3000.000000") "Undefined" 0 0))))
    (:then_1
      (if _isvalid_2
        (Variables|Default|SetTime%20until%20drop _returnvalue_2)))
    (:then_2
      (if _isvalid
        (Variables|Default|SetAmountOfDrops _returnvalue)))))

(fn ConstructionScript)

(fn CheckforStart
  (if (Variables|/Game/Mordhau/Blueprints/GameModes/BattleRoyale/BP_BattleRoyaleGameMode.BP_BattleRoyaleGameMode_C|GetInitializedMatch (Variables|Default|GetAs%20BP%20Battle%20Royale%20Game%20Mode))
    (Utilities|Time|ClearandInvalidateTimerbyHandle (Variables|Default|GetCheckerTimer))
    (CallFunction|AllAnnouncement (Utilities|Text|FormatText "== An airdrop will land in {a} seconds! ==" (Variables|Default|GetTime%20until%20drop)))
    (bind _returnvalue (Utilities|Time|SetTimerbyFunctionName 0 "SpawnAirdropFunc" (Variables|Default|GetTime%20until%20drop)))
    (Variables|Default|SetAirdropTimer _returnvalue)))

(fn SpawnAirdropFunc
  (if (not (== 0 (Variables|Default|GetAmountOfDrops)))
    (CallFunction|SRVAirdrop)
    (bind _result (Math|Integer|DecrementInt (Variables|Default|GetAmountOfDrops))
      (:%20%20
        (if (not (== 0 _result))
          (Utilities|Time|SetTimerbyFunctionName 0 "SpawnAirdropFunc" (Variables|Default|GetTime%20until%20drop)))))))

(fn GenerateAirdropLocation
  (bind _as_bp_battle_royale_game_mode (Variables|Default|GetAs%20BP%20Battle%20Royale%20Game%20Mode))
  (bind _battleroyalecircle (Variables|/Game/Mordhau/Blueprints/GameModes/BattleRoyale/BP_BattleRoyaleGameMode.BP_BattleRoyaleGameMode_C|GetBattleRoyaleCircle _as_bp_battle_royale_game_mode))
  (bind _returnvalue (Actor|GetActorOfClass "/BRExtras/Airdrops/BP_swiiftAirdropLocationForcer.BP_swiiftAirdropLocationForcer_C"))
  (Utilities|IsValid _returnvalue
    (:Is%20Valid
      (return (Transformation|GetActorLocation _returnvalue)))
    (:Is%20Not%20Valid
      (bind _subcirclecenter (Default|FindRandomCircleCenterInside _battleroyalecircle 2e+03 (Utilities|Array|Get(acopy) (Variables|/Game/Mordhau/Blueprints/GameModes/BattleRoyale/BP_BattleRoyaleCircle.BP_BattleRoyaleCircle_C|GetCircleCentersPerLevel _battleroyalecircle) (Math|Conversions|ToInteger(Byte) (+ (.currentcirclelevel (Variables|/Game/Mordhau/Blueprints/GameModes/BattleRoyale/BP_BattleRoyaleCircle.BP_BattleRoyaleCircle_C|GetCircleState _battleroyalecircle)) 1))) 1.0))
      (bind _returnvalue_2 (Actor|GetActorOfClass "/Script/Mordhau.MordhauCharacter"))
      (bind _randomlocation (Class|NavigationSystemV1|GetRandomLocationinNavigableRadius (Math|Vector|MakeVector (.X (Math|Vector|BreakVector _subcirclecenter)) (.Y (Math|Vector|BreakVector _subcirclecenter)) (.Z (Math|Vector|BreakVector (Transformation|GetActorLocation _returnvalue_2)))) 1e+02 0 "/Game/Mordhau/AI/Navigation/BP_NavFilter_NoLadder.BP_NavFilter_NoLadder_C"))
      (return _randomlocation))))

(fn SpawnAirdrop
  (params (Location :type Vector))
  (Game|SpawnActorfromClass "/BRExtras/Airdrops/BP_swiiftAirdrop.BP_swiiftAirdrop_C" (Math|Transform|MakeTransform Location) "Undefined" 0 0)
  (CallFunction|AllAnnouncement "=== AIRDROP SPAWNED! ==="))