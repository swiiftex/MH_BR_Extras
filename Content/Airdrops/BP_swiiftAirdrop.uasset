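; Mordhau airdrop actor that moves its skeletal mesh over TimeToDrop when play begins and passes interaction starts to its parent class.
; DropChest removes the widget, snaps the static mesh onto the skeletal mesh and turns on physics that ignores pawns.
; The delayed chain that would call DropChest and stop the move is disconnected, so that drop step never runs.
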(event EventOnInteractionStart
  (params (Character :type Mordhau%20Character%20Object%20Reference))
  (|CallParentFunction Character))

(event EventBeginPlay
  (Utilities|FlowControl|Sequence
    (:then_0
      (Components|MoveComponentTo (Variables|Default|GetSkeletalMesh) "0, 0, 0" "0, 0, 0" false false (Variables|Default|GetTimeToDrop) false))))

(fn ConstructionScript)

(fn DropChest
  (bind _skeletalmesh (Variables|Default|GetSkeletalMesh))
  (Components|DestroyComponent (Variables|Default|GetMordhauWidget1))
  (Transformation|AttachComponentToComponent (Variables|Default|GetStaticMesh) _skeletalmesh "None" "SnapToTarget" "SnapToTarget" "SnapToTarget" true)
  (Collision|SetCollisionEnabled _skeletalmesh "QueryAndPhysics")
  (Collision|SetCollisionObjectType _skeletalmesh "ECC_PhysicsBody")
  (Physics|SetSimulatePhysics _skeletalmesh true)
  (Collision|SetCollisionResponsetoChannel _skeletalmesh "ECC_Pawn" "ECR_Ignore"))