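; BP_AirdropProjectile is a projectile that delivers an airdrop where it hits.
; Its OnProjectileHit event spawns BP_swiiftAirdrop at the hit location with zero rotation and unit scale, adjusting for collisions but always spawning.
; The projectile then destroys itself, and the graph contains no other active logic.
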(event EventBeginPlay
  (|CallParentFunction) ; This node is disabled and will not be called.\nDrag off pins to build functionality.
)

(event Collision|EventActorBeginOverlap
  (params (OtherActor :type Actor%20Object%20Reference))
  (|CallParentFunction OtherActor) ; This node is disabled and will not be called.\nDrag off pins to build functionality.
)

(event EventTick
  (params (DeltaSeconds :type Float%20%28single-precision%29))
  (|CallParentFunction DeltaSeconds) ; This node is disabled and will not be called.\nDrag off pins to build functionality.
)

(event EventOnProjectileHit
  (params (HitLocation :type Vector :default "0, 0, 0") (HitNormal :type Vector :default "0, 0, 0") (BounceForce :type Float%20%28single-precision%29) (Surface :type Byte :default 0) (bHasHitWorld :type Boolean) (bHasStopped :type Boolean))
  (Game|SpawnActorfromClass "/BRExtras/Airdrops/BP_swiiftAirdrop.BP_swiiftAirdrop_C" (Math|Transform|MakeTransform HitLocation) "AdjustIfPossibleButAlwaysSpawn" 0 0)
  (Actor|DestroyActor))

(fn ConstructionScript
  (|CallParentFunction))