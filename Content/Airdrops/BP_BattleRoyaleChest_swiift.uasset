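; Breakable battle royale loot chest that opens when interacted with or damaged.
; BreakChest spawns a random item from each of three lists, removing picked classes from later lists, launches them with random impulses, and adds guaranteed items.
; The ChestDestroyed RepNotify toggles interaction, visibility and collision, playing break effects and spawning a ragdoll mesh.
; On authority, the chest then resets after RespawnTime, or expires if that is not positive.
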(event Custom|RespawnChest
  (Utilities|FlowControl|Delay (Variables|Default|GetRespawnTime))
  (Variables|Default|SetChestDestroyed false))

(event EventOnInteractionStart
  (params (Character :type Mordhau%20Character%20Object%20Reference))
  (Utilities|IsValid Character
    (:Is%20Valid
      (bind _asmordhau_player_controller (Utilities|Casting|CastToMordhauPlayerController (Pawn|GetController Character))
        (:then
          (CallFunction|BreakChest _asmordhau_player_controller))
        (:CastFailed
          (CallFunction|BreakChest))))))

(event Game|Damage|EventAnyDamage
  (params (Damage :type Float%20%28single-precision%29) (DamageType :type Damage%20Type%20Object%20Reference) (InstigatedBy :type Controller%20Object%20Reference) (DamageCauser :type Actor%20Object%20Reference))
  (bind _asmordhau_player_controller (Utilities|Casting|CastToMordhauPlayerController InstigatedBy)
    (:then
      (CallFunction|BreakChest _asmordhau_player_controller))
    (:CastFailed
      (CallFunction|BreakChest))))

(fn ConstructionScript)

(fn SpawnContents
  (params (CustomizeFor :type Mordhau%20Player%20Controller%20Object%20Reference))
  (bind _returnvalue (Math|Random|RandomFloatinRange -1.8e+02 1.8e+02))
  (bind _returnvalue_2 (Math|Vector|MakeVector 0.0 0.0 0.5))
  (bind _transformtouse (LocalVariables|GetTransformToUse))
  (bind _transformtouse_2 (LocalVariables|GetTransformToUse))
  (bind _returnvalue_3 (Math|Rotator|MakeRotator 0.0 0.0 _returnvalue))
  (bind _returnvalue_4 (Math|Vector|RotateVector "0.250000, 0, 0" _returnvalue_3))
  (bind _returnvalue_5 (+ _returnvalue_2 _returnvalue_4))
  (bind _returnvalue_6 (* _returnvalue_5 4.5e+02))
  (bind _returnvalue_7 (* _returnvalue_6 0.5))
  (if (not (Game|IsActorBeingDestroyed))
    (LocalVariables|SetOriginalFirstItemList (Variables|Default|GetItemList))
    (LocalVariables|SetOriginalSecondItemList (LocalVariables|GetOriginalSecondItemList))
    (LocalVariables|SetOriginalThirdItemList (LocalVariables|GetOriginalThirdItemList))
    (Utilities|Array|Add _transformtouse (Transformation|GetWorldTransform (Variables|Default|GetSpawnPoint1)))
    (Utilities|Array|Add _transformtouse (Transformation|GetWorldTransform (Variables|Default|GetSpawnPoint2)))
    (Utilities|Array|Add _transformtouse (Transformation|GetWorldTransform (Variables|Default|GetSpawnPoint3)))
    (LocalVariables|SetTransformIdx 0)
    (Utilities|FlowControl|Sequence
      (:then_0
        (for _index (range 0 2)
          (Utilities|FlowControl|Sequence
            (:then_0
              (switch int _index
                (:1
                  (Variables|Default|SetItemList (Variables|Spawning|GetSecondItemList)))
                (:2
                  (Variables|Default|SetItemList (Variables|Spawning|GetThirdItemList)))))
            (:then_1
              (bind _spawnedactor (CallFunction|SpawnRandomItem (Utilities|Array|Get(acopy) _transformtouse_2 (LocalVariables|GetTransformIdx)) CustomizeFor))
              (Utilities|IsValid _spawnedactor
                (:Is%20Valid
                  (Utilities|FlowControl|Sequence
                    (:then_0
                      (Math|Integer|IncrementInt (LocalVariables|GetTransformIdx)
                        (:%20%20
                          (bind _asmordhau_equipment (Utilities|Casting|CastToMordhauEquipment _spawnedactor)
                            (:then
                              (Variables|/Script/Mordhau.MordhauEquipment|SetbCanRagdoll _asmordhau_equipment true)
                              (Class|MordhauEquipment|UpdateEquipmentState _asmordhau_equipment)
                              (Utilities|IsValid (Variables|/Script/Mordhau.MordhauEquipment|GetPhysicsProxy _asmordhau_equipment)
                                (:Is%20Valid
                                  (bind _asskeletal_mesh_component (Utilities|Casting|CastToSkeletalMeshComponent (Variables|/Script/Engine.Actor|GetRootComponent (Variables|/Script/Mordhau.MordhauEquipment|GetPhysicsProxy _asmordhau_equipment))))
                                  (Physics|AddImpulse _asskeletal_mesh_component _returnvalue_6 "None" true)
                                  (Class|PrimitiveComponent|AddAngularImpulseinDegrees _asskeletal_mesh_component _returnvalue_7 "None" true))))
                            (:CastFailed
                              (bind _asbp_wearable_pickup (Utilities|Casting|CastToBP_WearablePickup _spawnedactor))
                              (Physics|AddImpulse (Variables|/Script/Mordhau.SkeletalMeshMordhauActor|GetSkeletalMeshComponent _asbp_wearable_pickup) _returnvalue_6 "None" true)
                              (Class|PrimitiveComponent|AddAngularImpulseinDegrees (Variables|/Script/Mordhau.SkeletalMeshMordhauActor|GetSkeletalMeshComponent _asbp_wearable_pickup) _returnvalue_7 "None" true))))))
                    (:then_1
                      (Utilities|Map|Remove (Variables|Spawning|GetSecondItemList) (Utilities|GetClass _spawnedactor))
                      (Utilities|Map|Remove (Variables|Spawning|GetThirdItemList) (Utilities|GetClass _spawnedactor)))))))))
        (for _array_element (Variables|Spawning|GetGuaranteedItems)
          (Game|SpawnActorfromClass _array_element (Utilities|Array|Get(acopy) _transformtouse_2) "AdjustIfPossibleButAlwaysSpawn" 0 0)))
      (:then_1
        (Variables|Default|SetItemList (LocalVariables|GetOriginalFirstItemList))
        (Variables|Spawning|SetSecondItemList (LocalVariables|GetOriginalSecondItemList))
        (Variables|Spawning|SetThirdItemList (LocalVariables|GetOriginalThirdItemList))))))

(fn OnRepDestroyed
  (bind _returnvalue (Transformation|GetActorLocation))
  (bind _chestdestroyed (Variables|Default|GetChestDestroyed))
  (bind _skeletalmesh (Variables|Default|GetSkeletalMesh))
  (bind _returnvalue_2 (Collision|GetCollisionEnabled _skeletalmesh))
  (Variables|Default|SetbIsInteractable (not _chestdestroyed))
  (Utilities|FlowControl|Sequence
    (:then_0
      (Development|SetHiddeninGame (Variables|Default|GetSkeletalMesh) _chestdestroyed false)
      (if _chestdestroyed
        (Utilities|FlowControl|Sequence
          (:then_0
            (if (Utilities|Enum|NotEqual(Enum) _returnvalue_2 "NoCollision")
              (Collision|SetCollisionEnabled _skeletalmesh "NoCollision")))
          (:then_1
            (Networking|CanExecuteCosmeticEvents
              (:True
                (Effects|SpawnEmitteratLocation (Variables|Default|GetDestroyedParticles) _returnvalue)
                (Audio|PlaySoundatLocation "/Game/Mordhau/Audio/Cues/Misc/SC_Chest_Break.SC_Chest_Break" _returnvalue "0, 0, 0" 1.0 1.0 0.0 0 0 0)
                (Utilities|IsValid (Variables|Default|GetDestroyedRagdollMesh)
                  (:Is%20Valid
                    (bind _returnvalue_3 (Game|SpawnActorfromClass "/Game/Mordhau/Blueprints/GameModes/BattleRoyale/BP_BattleRoyaleChestRagdoll.BP_BattleRoyaleChestRagdoll_C" (Transformation|GetActorTransform) "Undefined" 0 0))
                    (Class|SkinnedMeshComponent|SetSkeletalMesh (Variables|/Script/Engine.SkeletalMeshActor|GetSkeletalMeshComponent _returnvalue_3) (Variables|Default|GetDestroyedRagdollMesh) true)
                    (Collision|SetCollisionEnabled (Variables|/Script/Engine.SkeletalMeshActor|GetSkeletalMeshComponent _returnvalue_3) "QueryAndPhysics")
                    (Physics|SetSimulatePhysics (Variables|/Script/Engine.SkeletalMeshActor|GetSkeletalMeshComponent _returnvalue_3) true)))))))
        (elif (Utilities|Enum|NotEqual(Enum) _returnvalue_2 "QueryAndPhysics")
          (Collision|SetCollisionEnabled _skeletalmesh "QueryAndPhysics"))))
    (:then_1
      (if _chestdestroyed
        (CallFunction|OnChestDestroyed)
        (Networking|SwitchHasAuthority
          (:Authority
            (if (> (Variables|Default|GetRespawnTime) 0.0)
              (CallFunction|RespawnChest)
              (else
                (Actor|SetLifeSpan 2.0)))))))))

(fn OnChestDestroyed)

(fn BreakChest
  (params (DestroyerPlayerController :type Mordhau%20Player%20Controller%20Object%20Reference))
  (if (not (Variables|Default|GetChestDestroyed))
    (Collision|SetCollisionEnabled (Variables|Default|GetSkeletalMesh) "NoCollision")
    (CallFunction|SpawnContents DestroyerPlayerController)
    (Variables|Default|SetChestDestroyed true)))

(fn AddRandomImpulse
  (params (Target :type Primitive%20Component%20Object%20Reference))
  (bind _returnvalue (Math|Random|RandomFloatinRange -1.8e+02 1.8e+02))
  (bind _returnvalue_2 (Math|Vector|MakeVector 0.0 0.0 0.5))
  (bind _returnvalue_3 (Math|Rotator|MakeRotator 0.0 0.0 _returnvalue))
  (bind _returnvalue_4 (Math|Vector|RotateVector "0.250000, 0, 0" _returnvalue_3))
  (bind _returnvalue_5 (+ _returnvalue_2 _returnvalue_4))
  (bind _returnvalue_6 (* _returnvalue_5 4.5e+02))
  (Physics|AddImpulse Target _returnvalue_6 "None" true)
  (Class|PrimitiveComponent|AddAngularImpulseinDegrees Target (* _returnvalue_6 0.5) "None" true))