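; BP_ZoneProtectionZone is a temporary safe zone that shields Mordhau characters from the Battle Royale circle for a ten-second lifespan.
; Its capsule overlaps track characters inside, and every tick it removes them from the circle's UnsafeCharacters set.
; When a character leaves the capsule, it is added back to that set if it is not overlapping the circle's own capsule.
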(event OnComponentBeginOverlap(Capsule)
  (params (OverlappedComponent :type Primitive%20Component%20Object%20Reference) (OtherActor :type Actor%20Object%20Reference) (OtherComp :type Primitive%20Component%20Object%20Reference) (OtherBodyIndex :type Integer) (bFromSweep :type Boolean) (SweepResult :type Hit%20Result%20Structure%20%28by%20ref%29))
  (bind _asmordhau_character (Utilities|Casting|CastToMordhauCharacter OtherActor))
  (Utilities|Array|AddUnique (Variables|Default|GetCharsInside) _asmordhau_character))

(event OnComponentEndOverlap(Capsule)
  (params (OverlappedComponent :type Primitive%20Component%20Object%20Reference) (OtherActor :type Actor%20Object%20Reference) (OtherComp :type Primitive%20Component%20Object%20Reference) (OtherBodyIndex :type Integer))
  (bind _asmordhau_character (Utilities|Casting|CastToMordhauCharacter OtherActor))
  (Utilities|Array|RemoveItem (Variables|Default|GetCharsInside) _asmordhau_character)
  (if (== (Utilities|Array|FindItem (Collision|GetOverlappingActors (Variables|/Game/Mordhau/Blueprints/GameModes/BattleRoyale/BP_BattleRoyaleCircle.BP_BattleRoyaleCircle_C|GetCapsule (Variables|Default|GetCircleRef)) "/Script/Mordhau.AdvancedCharacter" :!class /Script/Engine.PrimitiveComponent) _asmordhau_character) -1)
    (Utilities|Set|Add (Variables|/Game/Mordhau/Blueprints/GameModes/BattleRoyale/BP_BattleRoyaleCircle.BP_BattleRoyaleCircle_C|GetUnsafeCharacters (Variables|Default|GetCircleRef)) _asmordhau_character)))

(event EventBeginPlay
  (Actor|SetLifeSpan 1e+01)
  (bind _returnvalue (Actor|GetActorOfClass "/Game/Mordhau/Blueprints/GameModes/BattleRoyale/BP_BattleRoyaleCircle.BP_BattleRoyaleCircle_C"))
  (Variables|Default|SetCircleRef _returnvalue))

(event EventTick
  (params (DeltaSeconds :type Float%20%28single-precision%29))
  (Utilities|Set|RemoveItems (Variables|/Game/Mordhau/Blueprints/GameModes/BattleRoyale/BP_BattleRoyaleCircle.BP_BattleRoyaleCircle_C|GetUnsafeCharacters (Variables|Default|GetCircleRef)) (Variables|Default|GetCharsInside)))

(fn ConstructionScript)