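; BP_SpecPlayerName is an actor that carries a W_SpecPlayer widget for an attached player character, by its name a spectator name tag.
; On BeginPlay it passes AttachedTo to the widget and caches that actor as a MordhauCharacter.
; A looping one-second timer then destroys the tag once the character is dead.
; An unconnected SetLifeSpan branch never runs.
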(event Custom|CustomEvent_0
  (if (Class|AdvancedCharacter|GetIsDead (Variables|Default|GetAs%20Mordhau%20Character))
    (Actor|DestroyActor)))

(event EventBeginPlay
  (bind _asw_spec_player (Utilities|Casting|CastToW_SpecPlayer (UserInterface|GetWidget (Variables|Default|GetWidget))))
  (bind _output_get (Variables|/BRExtras/W_SpecPlayer.W_SpecPlayer_C|SetAttachedActor _asw_spec_player (Variables|Default|GetAttachedTo)))
  (bind _asmordhau_character (Utilities|Casting|CastToMordhauCharacter _output_get))
  (Variables|Default|SetAs%20Mordhau%20Character _asmordhau_character)
  (Utilities|Time|SetTimerbyEvent (delegate Custom|CustomEvent_0) 1.0 true))

(fn ConstructionScript)