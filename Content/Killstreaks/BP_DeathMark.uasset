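; BP_DeathMark is a killstreak actor that shows a death mark widget for the Mordhau character it is attached to.
; On BeginPlay it passes the attached actor to its W_DeathMark widget, caches the character and sets its lifespan from a Length variable.
; A looping one-second timer destroys the mark early once that character is dead.
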(event Custom|CustomEvent_0
  (if (Class|AdvancedCharacter|GetIsDead (Variables|Default|GetAs%20Mordhau%20Character))
    (Actor|DestroyActor)))

(event EventBeginPlay
  (bind _asw_death_mark (Utilities|Casting|CastToW_DeathMark (UserInterface|GetWidget (Variables|Default|GetWidget))))
  (bind _output_get (Variables|/BRExtras/Killstreaks/W_DeathMark.W_DeathMark_C|SetAttachedActor _asw_death_mark (Variables|Default|GetAttachedTo)))
  (bind _asmordhau_character (Utilities|Casting|CastToMordhauCharacter _output_get))
  (Variables|Default|SetAs%20Mordhau%20Character _asmordhau_character)
  (Actor|SetLifeSpan (Variables|Default|GetLength))
  (Utilities|Time|SetTimerbyEvent (delegate Custom|CustomEvent_0) 1.0 true))

(fn ConstructionScript)