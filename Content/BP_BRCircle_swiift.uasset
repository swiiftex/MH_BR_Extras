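; Battle royale zone for Mordhau that shrinks through timed levels, damaging characters via the parent's DealDamage.
; ActivateCircle plans centres backwards from the final spot, a random BP_ZoneEndFixer if any exist.
; Tick advances levels on the server and lerps mesh and capsule by server time, while a timer re-sends level info, which ChangeZoneSpeed can rescale.
; At minimum radius it starts drifting randomly, then announces sudden death, draining everyone until one character remains.
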(event Custom|SRV%20Start%20Replicating%20Stuff
  (if (not (== (.CurrentCircleLevel (Utilities|Struct|BreakBP_BattleRoyaleCircleState (Variables|Default|GetCircleState))) 255))
    (CallFunction|MCReplicationRecieve (Variables|Default|GetCircleInfoPerLevel))))

(event Custom|CustomEvent_0
  (CallFunction|SRVStartReplicatingStuff))

(event Custom|MC%20Replication%20Recieve
  (params (CircleInfoPerLevel :type Array%20of%20BP%20Battle%20Royale%20Circle%20Info%20Structures))
  (Variables|Default|SetCircleInfoPerLevel CircleInfoPerLevel))

(event Custom|All%20Announcement
  (params (Text :type Text) (Text2 :type Text) (Subtext :type Text) (Duration :type Float%20%28single-precision%29))
  (Class|MordhauGameMode|Broadcast (.AsMordhau%20Game%20Mode (Utilities|Casting|CastToMordhauGameMode (Game|GetGameMode))) 0 (Utilities|String|ToString(Text) Text) "ServerSay")
  (bind _asbp_mordhau_hud (Utilities|Casting|CastToBP_MordhauHUD (HUD|GetHUD (Game|GetPlayerController 0))))
  (Default|ShowAnnouncement _asbp_mordhau_hud Text2 Subtext Duration "NewEnumerator0"))

(event Custom|Start%20Randomly%20Moving
  (Networking|SwitchHasAuthority
    (:Authority
      (Utilities|FlowControl|DoOnce false
        (:Completed
          (CallFunction|MoveRandom))))))

(event Custom|MoveRandom
  (bind _returnvalue (Math|Random|RandomUnitVector))
  (bind _endcirclebasespeed (Variables|Default|GetEndCircleBaseSpeed))
  (bind _returnvalue_2 (* _returnvalue _endcirclebasespeed))
  (Development|PrintText (Utilities|Text|FormatText "Moving zone to {a}" (Utilities|String|ToString(Vector) _returnvalue_2)))
  (Variables|Default|SetMovingEndCircleLocation (+ (Transformation|GetActorLocation) _returnvalue_2))
  (Variables|Default|SetEndCircleStartTime (GameState|GetServerWorldTimeSeconds (Game|GetGameState)))
  (Utilities|Time|SetTimerbyEvent (delegate Custom|CloseCircle) 2e+01))

(event Custom|CloseCircle
  (CallFunction|AllAnnouncement "== Sudden death in 10 seconds! ==" "Sudden Death" "in 10 seconds!" 9.0)
  (Utilities|FlowControl|Delay 1e+01)
  (CallFunction|MCSetMat)
  (bind _returnvalue (Utilities|Time|SetTimerbyFunctionName 0 "DamageEveryone" 0.1 true))
  (Variables|Default|SetDamagerTimer _returnvalue)
  (CallFunction|AllAnnouncement "== Sudden death! ==" "Sudden Death!" "" 1e+01))

(event Custom|MC%20Set%20Mat
  (Rendering|Material|SetMaterial (Variables|Default|GetStaticMesh) 0 "/BRExtras/BRZoneMaterial_Deadly.BRZoneMaterial_Deadly"))

(event Custom|On%20start
  (bind _circleinfoperlevel (Variables|Default|GetCircleInfoPerLevel))
  (Utilities|Array|SetArrayElem _circleinfoperlevel (Utilities|Array|LastIndex _circleinfoperlevel) (Utilities|Struct|MakeBP_BattleRoyaleCircleInfo 4e+02 999999.0 2 0.1)))

(event EventBeginPlay
  (Utilities|FlowControl|Delay 3.0)
  (|CallParentFunction)
  (Variables|Default|SetOriginalCircleInfo (Variables|Default|GetCircleInfoPerLevel))
  (Actor|DestroyActor (Variables|Default|GetCirclePostProcess))
  (Utilities|Time|SetTimerbyEvent (delegate Custom|CustomEvent_0) 1.0 true)
  (Variables|Default|SetMinCircleSize 4e+02))

(event Collision|EventActorBeginOverlap
  (params (OtherActor :type Actor%20Object%20Reference))
  (|CallParentFunction OtherActor) ; This node is disabled and will not be called.\nDrag off pins to build functionality.
)

(event EventTick
  (params (DeltaSeconds :type Float%20%28single-precision%29))
  (bind _returnvalue (Game|GetPlayerCameraManager 0))
  (bind _returnvalue_2 (Transformation|GetActorLocation))
  (bind _audio (Variables|Default|GetAudio))
  (bind _endcirclestarttime (Variables|Default|GetEndCircleStartTime))
  (bind _damageinterval (Variables|Default|GetDamageInterval))
  (bind _circlestate (Variables|Default|GetCircleState))
  (bind (_currentcirclelevel _circlestartservertime) (Utilities|Struct|BreakBP_BattleRoyaleCircleState _circlestate))
  (bind _returnvalue_3 (Transformation|GetActorLocation _returnvalue))
  (bind _asbp_battle_royale_game_state (Utilities|Casting|CastToBP_BattleRoyaleGameState (Game|GetGameState)))
  (if (not (Variables|/Game/Mordhau/Blueprints/GameModes/BP_MordhauGameState.BP_MordhauGameState_C|GetMatchEndInfoReplicated _asbp_battle_royale_game_state))
    (Utilities|FlowControl|Sequence
      (:then_0
        (Networking|SwitchHasAuthority
          (:Authority
            (Utilities|FlowControl|Sequence
              (:then_0
                (Utilities|FlowControl|DoOnce false
                  (:Completed
                    (CallFunction|OnStart))))
              (:then_1
                (Utilities|FlowControl|Sequence
                  (:then_0
                    (if (>= (Utilities|Time|GetTimeSeconds) (+ (.Duration (Utilities|Struct|BreakBP_BattleRoyaleCircleInfo (Utilities|Array|Get(acopy) (Variables|Default|GetCircleInfoPerLevel) (Math|Conversions|ToInteger(Byte) _currentcirclelevel)))) _circlestartservertime))
                      (CallFunction|BeginCircleLevel (+ _currentcirclelevel 1))))
                  (:then_1
                    (Variables|Default|SetDamageDealTick (+ (Variables|Default|GetDamageDealTick) DeltaSeconds))
                    (if (>= (Variables|Default|GetDamageDealTick) _damageinterval)
                      (Variables|Default|SetDamageDealTick (- (Variables|Default|GetDamageDealTick) _damageinterval))
                      (CallFunction|DealDamage)))))))))
      (:then_1
        (CallFunction|InterpCircle)
        (if (< (Components|Capsule|GetScaledCapsuleRadius (Variables|Default|GetCapsule)) 401.0)
          (CallFunction|StartRandomlyMoving)
          (if (not (Math|Vector|Equal(Vector) (Transformation|GetActorLocation) (Variables|Default|GetMovingEndCircleLocation) 1e+01))
            (bind _returnvalue_4 (Class|MordhauUtilityLibrary|GetNormalizedTime _endcirclestarttime (+ _endcirclestarttime 3e+01) (GameState|GetServerWorldTimeSeconds (Game|GetGameState))))
            (Transformation|SetActorLocation (Math|Vector|Lerp(Vector) (Transformation|GetActorLocation) (Variables|Default|GetMovingEndCircleLocation) _returnvalue_4) false false))))
      (:then_2
        (Networking|CanExecuteCosmeticEvents
          (:True
            (Utilities|FlowControl|Sequence
              (:then_0
                (Utilities|FlowControl|DoOnce false
                  (:Completed
                    (Components|Activation|Activate _audio false))))
              (:then_1
                (Transformation|SetWorldLocation _audio (Math|Conversions|ToVector(Vector2D) (+ (* (Math|Vector2D|Normalize2D (Math|Conversions|ToVector2D(Vector) (- _returnvalue_3 _returnvalue_2))) (Variables|/Script/Engine.CapsuleComponent|GetCapsuleRadius (Variables|Default|GetCapsule))) (Math|Conversions|ToVector2D(Vector) _returnvalue_2)) (.Z (Math|Vector|BreakVector _returnvalue_3))) false false)))))))))

(fn ConstructionScript
  (|CallParentFunction))

(fn DealDamage
  (bind _result (Utilities|Set|ToArray (Variables|Default|GetUnsafeCharacters)))
  (for _array_element _result
    (bind _asbp_swiift_brchar (Utilities|Casting|CastToBP_swiiftBRChar _array_element))
    (Variables|/BRExtras/BP_swiiftBRChar.BP_swiiftBRChar_C|SetInCircle? _asbp_swiift_brchar true))
  (bind _result_2 (Utilities|Set|ToArray (Variables|Default|GetSafeCharacters)))
  (for _array_element_2 _result_2
    (bind _asbp_swiift_brchar_2 (Utilities|Casting|CastToBP_swiiftBRChar _array_element_2))
    (Variables|/BRExtras/BP_swiiftBRChar.BP_swiiftBRChar_C|SetInCircle? _asbp_swiift_brchar_2 false))
  (|CallParentFunction))

(fn InterpCircle
  (bind _returnvalue (Game|GetGameState))
  (bind _circlestate (Variables|Default|GetCircleState))
  (bind _circleinfoperlevel (Variables|Default|GetCircleInfoPerLevel))
  (bind _staticmesh (Variables|Default|GetStaticMesh))
  (bind (_currentcirclelevel _circlestartservertime _circlestartlocation _circleendlocation) (Utilities|Struct|BreakBP_BattleRoyaleCircleState _circlestate))
  (bind _returnvalue_2 (Transformation|GetWorldScale _staticmesh))
  (bind _returnvalue_3 (Math|Conversions|ToInteger(Byte) _currentcirclelevel))
  (bind _z (Math|Vector|BreakVector _returnvalue_2))
  (bind _returnvalue_4 (+ _returnvalue_3 1))
  (bind _output (Utilities|Array|Get(acopy) _circleinfoperlevel _returnvalue_3))
  (bind (_radius _duration) (Utilities|Struct|BreakBP_BattleRoyaleCircleInfo _output))
  (bind _returnvalue_5 (* _radius 0.002))
  (Utilities|IsValid _returnvalue
    (:Is%20Valid
      (if (Utilities|Array|IsValidIndex _circleinfoperlevel _returnvalue_4)
        (LocalVariables|SetNextRadius (.Radius (Utilities|Struct|BreakBP_BattleRoyaleCircleInfo (Utilities|Array|Get(acopy) _circleinfoperlevel _returnvalue_4))))
        (else
          (LocalVariables|SetNextRadius 4e+02)))
      (bind _returnvalue_6 (Class|MordhauUtilityLibrary|GetNormalizedTime _circlestartservertime (+ _circlestartservertime _duration) (GameState|GetServerWorldTimeSeconds _returnvalue)))
      (Transformation|SetActorLocation (Math|Vector|Lerp(Vector) _circlestartlocation _circleendlocation _returnvalue_6) false false)
      (Transformation|SetWorldScale3D _staticmesh (Math|Vector|MakeVector (.x (Math|Vector|Lerp(Vector) (Math|Vector|MakeVector _returnvalue_5 _returnvalue_5 _z) (Math|Vector|MakeVector (* (LocalVariables|GetNextRadius) 0.002) (* (LocalVariables|GetNextRadius) 0.002) _z) _returnvalue_6)) (.y (Math|Vector|Lerp(Vector) (Math|Vector|MakeVector _returnvalue_5 _returnvalue_5 _z) (Math|Vector|MakeVector (* (LocalVariables|GetNextRadius) 0.002) (* (LocalVariables|GetNextRadius) 0.002) _z) _returnvalue_6)) (.z (Math|Vector|Lerp(Vector) (Math|Vector|MakeVector _returnvalue_5 _returnvalue_5 _z) (Math|Vector|MakeVector (* (LocalVariables|GetNextRadius) 0.002) (* (LocalVariables|GetNextRadius) 0.002) _z) _returnvalue_6))))
      (Components|Capsule|SetCapsuleRadius (Variables|Default|GetCapsule) (Math|Float|Lerp _radius (LocalVariables|GetNextRadius) _returnvalue_6) false))))

(fn ChangeZoneSpeed
  (params (ZoneSpeedMultiplier :type Float%20%28single-precision%29) (Ignore%20First%20Zone? :type Boolean))
  (bind _originalcircleinfo (Variables|Default|GetOriginalCircleInfo))
  (bind _output_get (Variables|Default|SetZoneSpeedMultiplier ZoneSpeedMultiplier))
  (Utilities|Array|Clear (LocalVariables|GetNewLocalVar_0))
  (for (_array_element _array_index) _originalcircleinfo
    (Utilities|Array|Add (LocalVariables|GetNewLocalVar_0) (select (select Ignore%20First%20Zone? (or (== _array_index 0) (== (Utilities|Array|LastIndex _originalcircleinfo) _array_index)) (== (Utilities|Array|LastIndex _originalcircleinfo) _array_index)) _array_element (Utilities|Struct|MakeBP_BattleRoyaleCircleInfo (.Radius (Utilities|Struct|BreakBP_BattleRoyaleCircleInfo _array_element)) (/ (.Duration (Utilities|Struct|BreakBP_BattleRoyaleCircleInfo _array_element)) _output_get) (Math|Float|Truncate (* (Math|Float|Clamp(Float) (/ (Math|Conversions|ToFloat(Integer) (.DamagePerTick (Utilities|Struct|BreakBP_BattleRoyaleCircleInfo _array_element))) (.DamageTickInterval (Utilities|Struct|BreakBP_BattleRoyaleCircleInfo _array_element))) 0.0 6e+01) 0.05)) 0.05))))
  (Variables|Default|SetCircleInfoPerLevel (LocalVariables|GetNewLocalVar_0)))

(fn BeginCircleLevel
  (params (NewLevel :type Byte :default 0))
  (|CallParentFunction NewLevel))

(fn InterpCircleCustom
  (bind _circlestate (Variables|Default|GetCircleState))
  (bind _lerpspeed (LocalVariables|GetLerpSpeed))
  (bind _circleinfoperlevel (Variables|Default|GetCircleInfoPerLevel))
  (bind (_currentcirclelevel _circlestartservertime _circlestartlocation _circleendlocation) (Utilities|Struct|BreakBP_BattleRoyaleCircleState _circlestate))
  (bind _returnvalue (Math|Conversions|ToInteger(Byte) _currentcirclelevel))
  (bind _returnvalue_2 (+ _returnvalue 1))
  (return (Math|Vector|Lerp(Vector) (Transformation|GetActorLocation) _circleendlocation _lerpspeed) (Math|Float|Lerp (Class|CapsuleComponent|GetUnscaledCapsuleRadius (Variables|Default|GetCapsule)) (.Radius (Utilities|Struct|BreakBP_BattleRoyaleCircleInfo (select (Utilities|Array|IsValidIndex _circleinfoperlevel _returnvalue_2) (Utilities|Array|Get(acopy) _circleinfoperlevel _returnvalue_2) (Utilities|Struct|MakeBP_BattleRoyaleCircleInfo 0.0 999999.0 20 1.0)))) _lerpspeed)))

(fn MovetoRandomLoc)

(fn DamageEveryone
  (Networking|SwitchHasAuthority
    (:Authority
      (bind _outactors (Actor|GetAllActorsOfClass "/Game/Mordhau/Blueprints/Characters/BP_MordhauCharacter.BP_MordhauCharacter_C"))
      (if (> (Utilities|Array|Length _outactors) 1)
        (for _array_element _outactors
          (Class|AdvancedCharacter|OffsetHealth _array_element -1 true)
          (if (<= (Class|StatComponent|GetStatValue (Variables|/Script/Mordhau.AdvancedCharacter|GetHealthStatComponent _array_element)) 1)
            (Game|Damage|ApplyDamage _array_element 1e+02 0 0 "/Engine/EngineDamageTypes/DmgTypeBP_Environmental.DmgTypeBP_Environmental_C")))
        (Development|PrintString "Hurt everyone")
        (else
          (Utilities|Time|ClearandInvalidateTimerbyHandle (Variables|Default|GetDamagerTimer)))))))

(fn ActivateCircle
  (bind _circlecentersperlevel (Variables|Default|GetCircleCentersPerLevel))
  (bind _circleinfoperlevel (Variables|Default|GetCircleInfoPerLevel))
  (bind _circleinfoperlevel_2 (Variables|Default|GetCircleInfoPerLevel))
  (bind _returnvalue (Utilities|Array|Length _circlecentersperlevel))
  (bind _output (Utilities|Array|Get(acopy) _circleinfoperlevel_2))
  (bind _output_2 (Utilities|Array|Get(acopy) _circlecentersperlevel))
  (bind _radius (Utilities|Struct|BreakBP_BattleRoyaleCircleInfo _output))
  (bind _returnvalue_2 (- _returnvalue 1))
  (Utilities|FlowControl|Sequence
    (:then_0
      ;[1 1 1] Find circle spots working backwards from final spot
      (for _array_element _circleinfoperlevel
        (Utilities|Array|Add :TargetArray _circlecentersperlevel))
      (Utilities|Array|SetArrayElem _circlecentersperlevel 0 (Transformation|GetActorLocation))
      (bind _subcirclecenter (CallFunction|FindRandomCircleCenterInside _radius _output_2 (.Radius (Utilities|Struct|BreakBP_BattleRoyaleCircleInfo (Utilities|Array|Get(acopy) _circleinfoperlevel _returnvalue_2)))))
      (bind (_actor _valid_) (CallFunction|GetClosestActortoLocation "/BRExtraMapsVanilla/BP_ZoneEndFixer.BP_ZoneEndFixer_C" _subcirclecenter)) ; jsut gets a random one
      (Utilities|Array|SetArrayElem _circlecentersperlevel _returnvalue_2 (select _valid_ (Transformation|GetActorLocation _actor) _subcirclecenter)) ; End circle loc
      (for _index (range 0 (- _returnvalue 3))
        (bind _desiredcirclecenter (CallFunction|FindRandomCircleBetweenCircles _radius _output_2 (.Radius (Utilities|Struct|BreakBP_BattleRoyaleCircleInfo (Utilities|Array|Get(acopy) _circleinfoperlevel_2 (+ (- (- _returnvalue 2) _index) 1)))) (Utilities|Array|Get(acopy) _circlecentersperlevel (+ (- (- _returnvalue 2) _index) 1)) (.Radius (Utilities|Struct|BreakBP_BattleRoyaleCircleInfo (Utilities|Array|Get(acopy) _circleinfoperlevel_2 (- (- _returnvalue 2) _index))))))
        (Utilities|Array|SetArrayElem _circlecentersperlevel (- (- _returnvalue 2) _index) _desiredcirclecenter)))
    (:then_1
      (CallFunction|BeginCircleLevel)
      (Collision|SetCollisionEnabled (Variables|Default|GetCapsule) "QueryOnly"))))

(fn GetClosestActortoLocation
  (params (Class%20Filter :type Actor%20Class%20Reference) (Location :type Vector))
  (bind _outactors (Actor|GetAllActorsOfClass Class%20Filter))
  (if (== (Utilities|Array|Length _outactors) 0)
    (return 0 false)
    (else
      (Development|PrintString (Utilities|String|ToString(Vector) (Transformation|GetActorLocation (.OutItem (Utilities|Array|Random _outactors)))))
      (return (.OutItem (Utilities|Array|Random _outactors)) true))))